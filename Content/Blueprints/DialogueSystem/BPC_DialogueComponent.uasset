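; Dialogue component that shows data-table-driven dialogue on screen, one line per Interaction event.
; The first interaction creates a W_DialogueWidget, and later ones update its name, line and border color.
; Each row supplies the next row, data table and end flag, forming a linked chain that can span tables.
; The interaction after an end-flagged row removes and clears the widget, keeping that row's next pointers for the following conversation.
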(event `/Game/Blueprints/Interactables/BPI_Interactable.Interaction`
  (if (`self.End Dialogue`)
    (`Widget.RemoveFromParent` (`self.DialogueRef`))
    (set `self.End Dialogue` false)
    (set `self.DialogueRef` null)
    (else
      (`/Engine/EditorBlueprintResources/StandardMacros.IsValid` (`self.DialogueRef`)
        (:`Is Valid`
          (bind _returnvalue (`|GetDataTableRow` (`self.Data Table`) (`self.Row Name`))
            (:`then`
              (bind (_name _line _nextrow _bordercolor _datatable _enddialogue) (break `/Game/Blueprints/DialogueSystem/S_DialogueInfo` _returnvalue))
              (`/Game/Widgets/W_DialogueWidget.UpdateDialogue` (`self.DialogueRef`) _name _line _bordercolor)
              (set `self.Row Name` _nextrow)
              (set `self.Data Table` _datatable)
              (set `self.End Dialogue` _enddialogue))))
        (:`Is Not Valid`
          (bind _returnvalue_2 (`|GetDataTableRow` (`self.Data Table`) (`self.Row Name`))
            (:`then`
              (bind (_name_2 _line_2 _nextrow_2 _bordercolor_2 _datatable_2 _enddialogue_2) (break `/Game/Blueprints/DialogueSystem/S_DialogueInfo` _returnvalue_2))
              (bind _returnvalue_3 (`|CreateWidget` "/Game/Widgets/W_DialogueWidget.W_DialogueWidget_C" null _name_2 _line_2 _bordercolor_2))
              (bind _output_get (set `self.DialogueRef` _returnvalue_3))
              (`UserWidget.AddToViewport` _output_get 0)
              (set `self.Row Name` _nextrow_2)
              (set `self.Data Table` _datatable_2)
              (set `self.End Dialogue` _enddialogue_2))))))))