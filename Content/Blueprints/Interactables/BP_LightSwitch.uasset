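; BP_LightSwitch is an interactable light switch that toggles a set of controlled lights on and off.
; Its Interaction event flips IsOn, then sets the visibility of each light component in the ControlledLights array to match.
; It also rolls the Cube1 mesh between two opposite angles to show the switch position.
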(event `/Game/Blueprints/Interactables/BPI_Interactable.Interaction`
  (bind _ison_ (`self.IsOn?`))
  (bind _cube1 (`self.Cube1`))
  (set `self.IsOn?` (not (`self.IsOn?`)))
  (for _array_element (`self.ControlledLights`)
    (`SceneComponent.SetVisibility` (`Light.LightComponent` _array_element) _ison_ false))
  (if _ison_
    (`SceneComponent.K2_SetRelativeRotation` _cube1 (`KismetMathLibrary.MakeRotator` 15.0) false false)
    (else
      (`SceneComponent.K2_SetRelativeRotation` _cube1 (`KismetMathLibrary.MakeRotator` -15.0) false false))))

(fn `UserConstructionScript`)