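; BP_ExtDoors is an interactable exterior door that moves the player to the L_World level.
; Its box trigger shows the HUD's interact widget while the player character overlaps it and removes it on exit, using a HUD reference cached at BeginPlay.
; The Interaction event fades the camera to black, waits for the fade, then opens L_World.
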(event `self.ReceiveBeginPlay`
  (bind _asbp_hud (cast `/Game/Widgets/BP_HUD` (`PlayerController.GetHUD` (`PlayerState.GetPlayerController` (`GameplayStatics.GetPlayerState` 0)))))
  (set `self.HUDRef` _asbp_hud))

(event `/Game/Blueprints/Interactables/BPI_Interactable.Interaction`
  (`PlayerCameraManager.StartCameraFade` :`self` (`GameplayStatics.GetPlayerCameraManager` 0) :`ToAlpha` 1.0 :`Duration` 0.5 :`bHoldWhenFinished` true)
  (`KismetSystemLibrary.Delay` 0.5)
  (`GameplayStatics.OpenLevel` "L_World"))

(event `self.Box.OnComponentBeginOverlap`
  (params (OverlappedComponent :type "PrimitiveComponent Object Reference") (OtherActor :type "Actor Object Reference") (OtherComp :type "PrimitiveComponent Object Reference") (OtherBodyIndex :type Integer) (bFromSweep :type Boolean) (SweepResult :type "HitResult Structure (by ref)"))
  (if (== OtherActor (`GameplayStatics.GetPlayerCharacter` 0))
    (`UserWidget.AddToViewport` (`/Game/Widgets/BP_HUD.InteractRef` (`self.HUDRef`)) 0)))

(event `self.Box.OnComponentEndOverlap`
  (params (OverlappedComponent :type "PrimitiveComponent Object Reference") (OtherActor :type "Actor Object Reference") (OtherComp :type "PrimitiveComponent Object Reference") (OtherBodyIndex :type Integer))
  (if (== (`GameplayStatics.GetPlayerCharacter` 0) OtherActor)
    (`Widget.RemoveFromParent` (`/Game/Widgets/BP_HUD.InteractRef` (`self.HUDRef`)))))

(fn `UserConstructionScript`)