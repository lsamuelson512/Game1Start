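; Interactable hinged door that swings open or closed on alternate Interaction calls, using a timeline played forward or in reverse.
; DoorMove lerps the root's yaw from its starting value to that plus 90 degrees when OpenRight is set, otherwise to the negation of that sum.
; Box overlap shows and removes the HUD's interact prompt for the player, with new prompts suppressed once the door first moves.
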(event `self.ReceiveBeginPlay`
  (bind (_returnvalue_roll _returnvalue_pitch _returnvalue_yaw) (`KismetMathLibrary.BreakRotator` (`SceneComponent.K2_GetComponentRotation` (`self.DefaultSceneRoot`))))
  (set `self.StrartingValue` _returnvalue_yaw)
  (bind _asbp_hud (cast `/Game/Widgets/BP_HUD` (`PlayerController.GetHUD` (`PlayerState.GetPlayerController` (`GameplayStatics.GetPlayerState` 0)))))
  (set `self.HUDRef` _asbp_hud))

(event `/Game/Blueprints/Interactables/BPI_Interactable.Interaction`
  (`/Engine/EditorBlueprintResources/StandardMacros.FlipFlop`
    (:`A`
      (bind (_direction _newtrack_0) (`Timeline|DoorMovement` :!label _label)
        (:`Update`
          (`self.DoorMove` _newtrack_0))))
    (:`B`
      (goto _label :!via `Reverse`))))

(event `self.Box.OnComponentBeginOverlap`
  (params (OverlappedComponent :type "PrimitiveComponent Object Reference") (OtherActor :type "Actor Object Reference") (OtherComp :type "PrimitiveComponent Object Reference") (OtherBodyIndex :type Integer) (bFromSweep :type Boolean) (SweepResult :type "HitResult Structure (by ref)"))
  (if (and (== OtherActor (`GameplayStatics.GetPlayerCharacter` 0)) (not (`self.Opened?`)))
    (`UserWidget.AddToViewport` (`/Game/Widgets/BP_HUD.InteractRef` (`self.HUDRef`)) 0)))

(event `self.Box.OnComponentEndOverlap`
  (params (OverlappedComponent :type "PrimitiveComponent Object Reference") (OtherActor :type "Actor Object Reference") (OtherComp :type "PrimitiveComponent Object Reference") (OtherBodyIndex :type Integer))
  (if (== (`GameplayStatics.GetPlayerCharacter` 0) OtherActor)
    (`Widget.RemoveFromParent` (`/Game/Widgets/BP_HUD.InteractRef` (`self.HUDRef`)))))

(fn `DoorMove`
  (params (Alpha :type "Float (double-precision)"))
  (bind _strartingvalue (`self.StrartingValue`))
  (bind _defaultsceneroot (`self.DefaultSceneRoot`))
  (bind _returnvalue (+ _strartingvalue 90.0))
  (if (`self.OpenRight?`)
    (`SceneComponent.K2_SetWorldRotation` _defaultsceneroot (`KismetMathLibrary.MakeRotator` 0.0 0.0 (`KismetMathLibrary.Lerp` _strartingvalue _returnvalue Alpha)) false false)
    (else
      (`SceneComponent.K2_SetWorldRotation` _defaultsceneroot (`KismetMathLibrary.MakeRotator` 0.0 0.0 (`KismetMathLibrary.Lerp` _strartingvalue (* _returnvalue -1.0) Alpha)) false false)))
  (`/Engine/EditorBlueprintResources/StandardMacros.DoOnce` false
    (:`Completed`
      (set `self.Opened?` true))))

(fn `UserConstructionScript`)